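; Game manager for a tic-tac-toe match that owns the board state, its X/O text displays and the game-over flag.
; SetGridSpace stores a mark as 1 or -1, updates that cell's text and runs CheckForVictory, which calls GameOver on a winning line.
; Win checks sum WinningRows index triples, so CheckForPossibleVictory can match a given sum and return the empty cell that completes that line.
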(event `self.ReceiveTick`
  (params (DeltaSeconds :type "Float (single-precision)")))

(fn `CheckForPossibleVictory`
  (params (check :type Integer))
  (returns (indexToWin :type Integer) (possible :type Boolean))
  (locals (index :type Integer))
  (bind _index (`local.index`))
  (bind _output (`|GetArrayItem` (`self.winningRows`) (+ _index 0)))
  (bind _output_2 (`|GetArrayItem` (`self.winningRows`) (+ _index 2)))
  (bind _output_3 (`|GetArrayItem` (`self.winningRows`) (+ _index 1)))
  (bind _output_4 (`|GetArrayItem` (`self.grid`) _output_2))
  (bind _output_5 (`|GetArrayItem` (`self.grid`) _output))
  (bind _output_6 (`|GetArrayItem` (`self.grid`) _output_3))
  (`KismetSystemLibrary.PrintString` "Checking for potential victory" :!label _label)
  (`KismetSystemLibrary.PrintString` (`KismetStringLibrary.Conv_IntToString` _output))
  (`KismetSystemLibrary.PrintString` (`KismetStringLibrary.Conv_IntToString` _output_3))
  (`KismetSystemLibrary.PrintString` (`KismetStringLibrary.Conv_IntToString` _output_2))
  ;[1 1 1] if array[index] + array[index+1] + array[index+2] == [CHECK]
  (if (== check (+ _output_5 _output_6 _output_4 0))
    (if (== _output_5 0)
      (return _output true)
      (elif (== _output_6 0)
        (return _output_3 true)
        (elif (== 0 _output_4)
          (return _output_2 true))))
    (else
      ;[1 1 1] index += 3
      (set `local.index` (+ (`local.index`) 3))
      (`KismetSystemLibrary.PrintString` (`KismetStringLibrary.Conv_IntToString` (`local.index`)))
      (if (>= (`local.index`) 24)
        (return 0 false)
        (else
          (`KismetSystemLibrary.PrintString` "Looking for the next set")
          (`KismetSystemLibrary.PrintString` "Looking for the next set")
          (goto _label))))))

(fn `CheckForVictory`
  (locals (index :type Integer) (total :type Integer))
  (bind _index (`local.index`))
  (bind _returnvalue (+ (`|GetArrayItem` (`self.grid`) (`|GetArrayItem` (`self.winningRows`) (+ _index 0))) (`|GetArrayItem` (`self.grid`) (`|GetArrayItem` (`self.winningRows`) (+ _index 1))) (`|GetArrayItem` (`self.grid`) (`|GetArrayItem` (`self.winningRows`) (+ _index 2))) 0))
  (`KismetSystemLibrary.PrintString` "Checking For Victory" :!label _label)
  ;[1 1 1] if array[index] + array[index+1] + array[index+2] == 3 or -3
  (if (or (== _returnvalue 3) (== _returnvalue -3))
    ;[1 1 1] Someone won, end the game
    (set `local.total` _returnvalue)
    (`self.GameOver`)
    (else
      ;[1 1 1] index += 3
      (set `local.index` (+ (`local.index`) 3))
      (`KismetSystemLibrary.PrintString` "no winner yet")
      (if (>= (`local.index`) 24)
        (`KismetSystemLibrary.PrintString` "No winner, keep playing")
        (return)
        (else
          (`KismetSystemLibrary.PrintString` "Looking for the next set")
          (goto _label))))))

(fn `GameOver`
  (`KismetSystemLibrary.PrintString` "We have a winner" true true (struct :`R` 1.0 :`B` 0.552721 :`A` 1.0) 20.0)
  (set `self.isgameOver` true))

(fn `IsSpaceEmpty`
  (params (index :type Integer))
  (returns (isEmpty :type Boolean))
  (if (== (`|GetArrayItem` (`self.grid`) index) 0)
    (return true)
    (else
      (return false))))

(fn `SetGridSpace`
  (params (index :type Integer) (mark :type Integer))
  (locals (i :type Integer))
  (`KismetArrayLibrary.Array_Set` (`self.grid`) index mark)
  (if (== mark 1)
    (`TextRenderComponent.K2_SetText` (`TextRenderActor.TextRender` (`|GetArrayItem` (`self.texts`) index)) "X")
    (`self.CheckForVictory` :!label _label)
    (elif (== mark -1)
      (`TextRenderComponent.K2_SetText` (`TextRenderActor.TextRender` (`|GetArrayItem` (`self.texts`) index)) "O")
      (goto _label))))

(fn `UserConstructionScript`)
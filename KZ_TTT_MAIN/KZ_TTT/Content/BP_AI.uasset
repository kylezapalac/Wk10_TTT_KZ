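; BP_AI is the computer opponent for a tic-tac-toe game, placing -1 marks through a Manager reference.
; MakeMove follows fixed priorities: win, block the player, take center, take a corner, then any space.
; A winning move calls GameOver, while other moves return the turn to the player.
; The corner search ignores its bottom-right emptiness check, always falling back to 8, and the "random" fallback picks the first empty space.
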(fn `ChooseRandomSpace`
  (returns (RandomOpenIndex :type Integer))
  (locals (temp :type Integer) (index :type Integer))
  (for _index (range 9)
    (bind _isempty (`/Game/BP_GameManager.IsSpaceEmpty` (`self.manager`) _index))
    (if _isempty
      (return _index))))

(fn `FindEmptyCorner`
  (returns (OpenCornerIndex :type Integer))
  (bind _manager (`self.manager`))
  ;[1 1 1] Check Top Left Corner
  (bind _isempty (`/Game/BP_GameManager.IsSpaceEmpty` _manager 0))
  (if _isempty
    (return 0)
    (else
      ;[1 1 1] Check Top Right Corner
      (bind _isempty_2 (`/Game/BP_GameManager.IsSpaceEmpty` _manager 2))
      (if _isempty_2
        (return 2)
        (else
          ;[1 1 1] Check Bottom Left Corner
          (bind _isempty_3 (`/Game/BP_GameManager.IsSpaceEmpty` _manager 6))
          (if _isempty_3
            (return 6)
            (else
              ;[1 1 1] Check Bottom Right Corner
              (`/Game/BP_GameManager.IsSpaceEmpty` _manager 8)
              (if true
                (return 8)
                (else
                  ;[1 1 1] No Corners Available
                  (return -1))))))))))

(fn `MakeMove`
  (locals (index :type Integer) (temp :type Integer))
  (bind _manager (`self.manager`))
  (bind _manager_2 (`self.manager`))
  (bind _manager_3 (`self.manager`))
  ;[1 1 1] Attempt to Win
  (bind (_indextowin _possible) (`/Game/BP_GameManager.CheckForPossibleVictory` _manager_2 -2))
  (if _possible
    (`/Game/BP_GameManager.SetGridSpace` _manager_2 _indextowin -1)
    (`/Game/BP_GameManager.GameOver` _manager_2)
    (else
      ;[1 1 1] Stop Player From Winning
      (bind (_indextowin_2 _possible_2) (`/Game/BP_GameManager.CheckForPossibleVictory` _manager_3 2))
      (if _possible_2
        (`/Game/BP_GameManager.SetGridSpace` _manager_3 _indextowin_2 -1)
        (else
          ;[1 1 1] Take Center Spot
          (bind _isempty (`/Game/BP_GameManager.IsSpaceEmpty` _manager 4))
          (if _isempty
            (`/Game/BP_GameManager.SetGridSpace` _manager 4 -1)
            (else
              ;[1 1 1] Take a Corner
              (bind _opencornerindex (`self.FindEmptyCorner`))
              (if (> _opencornerindex 0)
                (`/Game/BP_GameManager.SetGridSpace` (`self.manager`) _opencornerindex -1)
                (else
                  ;[1 1 1] Choose Random Spot
                  (bind _randomopenindex (`self.ChooseRandomSpace`))
                  (`/Game/BP_GameManager.SetGridSpace` (`self.manager`) _randomopenindex -1)))))))
      ;[1 1 1] End Turn
      (set `/Game/BP_GameManager.isPlayerTurn` true (`self.manager`))
      (return))))

(fn `UserConstructionScript`)
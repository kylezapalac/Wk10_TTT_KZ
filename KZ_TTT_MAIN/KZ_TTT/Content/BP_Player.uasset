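; Player Blueprint for a turn-based grid game against an AI, letting the player pick a space by looking at its block.
; Each Tick, a forward Visibility line trace finds actors tagged "Block" and stores their index from the Manager's Blocks array as Highlighted, or clears it.
; Pressing Activate on the player's turn marks that space through the Manager if empty, then passes the turn to the AI unless the game is over.
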(event `self.ReceiveTick`
  (params (DeltaSeconds :type "Float (single-precision)"))
  (bind _returnvalue (`self.K2_GetActorLocation`))
  ;[1 1 1] Do a RayCast
  (bind (_outhit _returnvalue_2) (`KismetSystemLibrary.LineTraceSingle` :`Start` _returnvalue :`End` (+ _returnvalue (* (`KismetMathLibrary.GetForwardVector` (`self.K2_GetActorRotation`)) (`self.rayDist`))) :`TraceChannel` "TraceTypeQuery1" :`DrawDebugType` "ForOneFrame"))
  ;[1 1 1] did we hit anything?
  (if _returnvalue_2
    (bind (_bblockinghit _binitialoverlap _time _distance _location _impactpoint _normal _impactnormal _physmat _hitactor) (`GameplayStatics.BreakHitResult` _outhit))
    ;[1 1 1] did we hit the right thing?
    (if (`self.ActorHasTag` _hitactor "Block")
      ;[1 1 1] if so, "highlight" the one we hit
      (for (_array_element _array_index) (`/Game/BP_GameManager.blocks` (`self.manager`))
        (if (== _array_element _hitactor)
          (set `self.highlighted` _array_index)))
      (else
        ;[1 1 1] if not, don't highlight anything
        (set `self.highlighted` -1 :!label _label)))
    (else
      (goto _label))))

(event `InputAction|Activate`
  (params (Key :type "Key Structure"))
  (bind _highlighted (`self.highlighted`))
  (bind _manager (`self.manager`))
  ;[1 1 1] if we press the button on our turn
  (:`Pressed`
    (if (`/Game/BP_GameManager.isPlayerTurn` (`self.manager`))
      ;[1 1 1] and if we have something selected
      (if (!= (`self.highlighted`) -1)
        ;[1 1 1] get the selected one
        (for (_ _array_index) (`/Game/BP_GameManager.grid` (`self.manager`))
          (if (== _array_index _highlighted)
            (bind _isempty (`/Game/BP_GameManager.IsSpaceEmpty` _manager _highlighted))
            (if _isempty
              (`/Game/BP_GameManager.SetGridSpace` _manager (`self.highlighted`) 1)
              ;[1 1 1] Switch to AI turn
              (set `/Game/BP_GameManager.isPlayerTurn` false (`self.manager`))
              (if (not (`/Game/BP_GameManager.isgameOver` (`self.manager`)))
                (`/Game/BP_AI.MakeMove` (`self.ai`)))
              (else
                (`KismetSystemLibrary.PrintString` "not valid")))))))))

(fn `UserConstructionScript`)